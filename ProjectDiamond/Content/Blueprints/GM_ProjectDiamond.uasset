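; GM_ProjectDiamond is the game mode Blueprint that handles checkpoint-based player respawning.
; RespawnPlayer destroys the current player character, then spawns a new BP_FPS_Character at the location and rotation of LastCheckpoint's POS component.
; Without a valid checkpoint, it spawns at the default transform instead of a player start.
; In both cases player controller 0 possesses the new character, and spawning ignores collisions.
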(event Custom|RespawnPlayer
  (Actor|DestroyActor (Game|GetPlayerCharacter 0))
  (bind _lastcheckpoint (Variables|Default|GetLastCheckpoint)
    (:then
      (bind _returnvalue (Game|SpawnActorfromClass "/Game/Blueprints/BP_FPS_Character.BP_FPS_Character_C" (Math|Transform|MakeTransform (.location (Transformation|GetWorldTransform (Variables|Default|GetPOS _lastcheckpoint))) (.rotation (Transformation|GetWorldTransform (Variables|Default|GetPOS _lastcheckpoint))) "1.000000,1.000000,1.000000") "AlwaysSpawn" "MultiplyWithRoot" 0 0))
      (Pawn|Possess (Game|GetPlayerController 0) _returnvalue))
    (:else
      (bind _returnvalue_2 (Game|SpawnActorfromClass "/Game/Blueprints/BP_FPS_Character.BP_FPS_Character_C" (Math|Transform|MakeTransform "0, 0, 0" "0, 0, 0" "1.000000,1.000000,1.000000") "AlwaysSpawn" "MultiplyWithRoot" 0 0))
      (Pawn|Possess (Game|GetPlayerController 0) _returnvalue_2))))

(event EventBeginPlay)

(event EventTick
  (params (DeltaSeconds :type Float%20%28single-precision%29)))

(fn ConstructionScript)