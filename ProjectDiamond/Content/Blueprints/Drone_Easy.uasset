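; Drone_Easy is a drone Blueprint that animates its Drone mesh with a hovering bob.
; On BeginPlay, the Drone_Bobbing timeline plays and lerps the mesh's relative Z between two heights.
; The construction script is empty, and disconnected nodes for adding a duplicate mesh with outline materials never run.
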(event EventBeginPlay
  (Utilities|FlowControl|Sequence
    (:then_0
      (bind _alpha (Timeline|Drone_Bobbing PlayFromStart)
        (:Update
          (Transformation|SetRelativeLocation (Variables|Default|GetDrone) (Math|Vector|MakeVector 0.0 0.0 (Math|Float|Lerp 0.0 5e+01 _alpha)) false false))))))

(fn ConstructionScript)