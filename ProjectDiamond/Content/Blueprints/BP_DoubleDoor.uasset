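; BP_DoubleDoor is a sliding double door that opens when the player's BP_FPS_Character enters its Box trigger.
; A DoOnce limits the opening to a single time, and the graph has no logic to close the door.
; Two timelines play together, each lerping one panel's relative X location so DDLeft and DDRight slide apart in opposite directions.
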(event OnComponentBeginOverlap(Box)
  (params (OverlappedComponent :type Primitive%20Component%20Object%20Reference) (OtherActor :type Actor%20Object%20Reference) (OtherComp :type Primitive%20Component%20Object%20Reference) (OtherBodyIndex :type Integer) (bFromSweep :type Boolean) (SweepResult :type Hit%20Result%20Structure%20%28by%20ref%29))
  (Utilities|Casting|CastToBP_FPS_Character OtherActor)
  (Utilities|FlowControl|DoOnce false
    (:Completed
      (Utilities|FlowControl|Sequence
        (:then_0
          (bind _alpha (Timeline|Timeline PlayFromStart)
            (:Update
              (Transformation|SetRelativeLocation (Variables|Default|GetDDLeft) (Math|Vector|MakeVector (Math|Float|Lerp 0.0 -1.6e+02 _alpha) 0.0 0.0) false false))))
        (:then_1
          (bind _alpha_2 (Timeline|Timeline_0 PlayFromStart)
            (:Update
              (Transformation|SetRelativeLocation (Variables|Default|GetDDRight) (Math|Vector|MakeVector (Math|Float|Lerp 0.0 1.6e+02 _alpha_2) 0.0 0.0) false false))))))))

(event EventBeginPlay)

(fn ConstructionScript)