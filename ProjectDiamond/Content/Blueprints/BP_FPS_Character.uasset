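; First-person player character for a speedrun-style parkour game, with double jump, dash, crouch slide, wall run and grappling hook, plus a timer widget.
; Overlap volumes detect "WallRun"-tagged actors, driving timelines that lock velocity along the wall and roll the camera; jumping launches away from it.
; Grapple line-traces from the camera, then Tick applies steerable pull force and updates the cable.
; Tick also plays headbob shakes, while a looping delay saves the last grounded location.
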(event OnComponentBeginOverlap(DetectWallCapsule)
  (params (OverlappedComponent :type Primitive%20Component%20Object%20Reference) (OtherActor :type Actor%20Object%20Reference) (OtherComp :type Primitive%20Component%20Object%20Reference) (OtherBodyIndex :type Integer) (bFromSweep :type Boolean) (SweepResult :type Hit%20Result%20Structure%20%28by%20ref%29))
  (bind _returnvalue (Transformation|GetActorForwardVector OtherActor))
  ;[1 0.3176 0.2471] Wall run logic
  (if (and (Actor|ActorHasTag OtherActor "WallRun") (AI|Components|NavMovement|IsFalling (Variables|Character|GetCharacterMovement)))
    (Utilities|FlowControl|Sequence
      (:then_0
        (CallFunction|ResetJump))
      (:then_1
        (Variables|Default|SetWall OtherActor)
        (Variables|Default|SetIsWallRunning true)
        (Variables|Default|SetPlayerDirection (* _returnvalue (Math|Integer|SelectInt 1 -1 (> (Math|Vector|DotProduct _returnvalue (Math|Vector|GetForwardVector (Variables|Default|GetCamera))) 0.0))))
        (Class|MovementComponent|SetPlaneConstraintNormal (Variables|Character|GetCharacterMovement) "0.000000,0.000000,1.000000")
        (Variables|/Script/Engine.CharacterMovementComponent|SetGravityScale (Variables|Character|GetCharacterMovement) 0.0)
        (Timeline|WallRunTimeline Play
          (:Update
            (Variables|/Script/Engine.MovementComponent|SetVelocity (Variables|Character|GetCharacterMovement) (* (Variables|Default|GetPlayerDirection) 1e+03))))))))

(event OnComponentEndOverlap(DetectWallCapsule)
  (params (OverlappedComponent :type Primitive%20Component%20Object%20Reference) (OtherActor :type Actor%20Object%20Reference) (OtherComp :type Primitive%20Component%20Object%20Reference) (OtherBodyIndex :type Integer))
  ;[1 0.3176 0.2471] Wall run logic
  (Variables|Default|SetWall 0)
  (if (Actor|ActorHasTag OtherActor "WallRun")
    (Utilities|FlowControl|Sequence
      (:then_0
        (Timeline|WallRunTimeline Stop
          (:Update
            (Variables|/Script/Engine.MovementComponent|SetVelocity (Variables|Character|GetCharacterMovement) (* (Variables|Default|GetPlayerDirection) 1e+03)))))
      (:then_1
        (Class|MovementComponent|SetPlaneConstraintNormal (Variables|Character|GetCharacterMovement) "0, 0, 0")
        (Variables|Default|SetIsWallRunning false)
        (Variables|/Script/Engine.CharacterMovementComponent|SetGravityScale (Variables|Character|GetCharacterMovement) (Variables|Default|GetOldGravityScale))))))

(event OnComponentBeginOverlap(WallDetectRight)
  (params (OverlappedComponent :type Primitive%20Component%20Object%20Reference) (OtherActor :type Actor%20Object%20Reference) (OtherComp :type Primitive%20Component%20Object%20Reference) (OtherBodyIndex :type Integer) (bFromSweep :type Boolean) (SweepResult :type Hit%20Result%20Structure%20%28by%20ref%29))
  (bind _returnvalue (Game|GetPlayerController 0))
  (bind _returnvalue_2 (Pawn|GetControlRotation _returnvalue :!class /Script/Engine.Controller))
  ;[1 1 1] Rotate Camera on Wall Run
  ;;[0.3075 0.8187 1] Rotate Right
  (if (and (Actor|ActorHasTag OtherActor "WallRun") (AI|Components|NavMovement|IsFalling (Variables|Character|GetCharacterMovement)))
    (bind _alpha (Timeline|RotateCameraRightTimeline Play)
      (:Update
        (Pawn|SetControlRotation _returnvalue (Math|Rotator|MakeRotator (Math|Float|Lerp (.roll (Transformation|GetActorRotation)) -2e+01 _alpha) (.pitch _returnvalue_2) (.yaw _returnvalue_2)))))))

(event OnComponentEndOverlap(WallDetectRight)
  (params (OverlappedComponent :type Primitive%20Component%20Object%20Reference) (OtherActor :type Actor%20Object%20Reference) (OtherComp :type Primitive%20Component%20Object%20Reference) (OtherBodyIndex :type Integer))
  (bind _returnvalue (Game|GetPlayerController 0))
  (bind _returnvalue_2 (Pawn|GetControlRotation _returnvalue :!class /Script/Engine.Controller))
  ;[1 1 1] Rotate Camera on Wall Run
  ;;[0.3075 0.8187 1] Rotate Right
  (if (Actor|ActorHasTag OtherActor "WallRun")
    (bind _alpha (Timeline|RotateCameraRightTimeline Reverse)
      (:Update
        (Pawn|SetControlRotation _returnvalue (Math|Rotator|MakeRotator (Math|Float|Lerp (.roll (Transformation|GetActorRotation)) -2e+01 _alpha) (.pitch _returnvalue_2) (.yaw _returnvalue_2)))))))

(event OnComponentBeginOverlap(WallDetectLeft)
  (params (OverlappedComponent :type Primitive%20Component%20Object%20Reference) (OtherActor :type Actor%20Object%20Reference) (OtherComp :type Primitive%20Component%20Object%20Reference) (OtherBodyIndex :type Integer) (bFromSweep :type Boolean) (SweepResult :type Hit%20Result%20Structure%20%28by%20ref%29))
  (bind _returnvalue (Game|GetPlayerController 0))
  (bind _returnvalue_2 (Pawn|GetControlRotation _returnvalue :!class /Script/Engine.Controller))
  ;[1 1 1] Rotate Camera on Wall Run
  ;;[0.4294 0.7963 1] Rotate Left
  (if (and (Actor|ActorHasTag OtherActor "WallRun") (AI|Components|NavMovement|IsFalling (Variables|Character|GetCharacterMovement)))
    (bind _alpha (Timeline|RotateCameraLeftTimeline Play)
      (:Update
        (Pawn|SetControlRotation _returnvalue (Math|Rotator|MakeRotator (Math|Float|Lerp (.roll (Transformation|GetActorRotation)) 2e+01 _alpha) (.pitch _returnvalue_2) (.yaw _returnvalue_2)))))))

(event OnComponentEndOverlap(WallDetectLeft)
  (params (OverlappedComponent :type Primitive%20Component%20Object%20Reference) (OtherActor :type Actor%20Object%20Reference) (OtherComp :type Primitive%20Component%20Object%20Reference) (OtherBodyIndex :type Integer))
  (bind _returnvalue (Game|GetPlayerController 0))
  (bind _returnvalue_2 (Pawn|GetControlRotation _returnvalue :!class /Script/Engine.Controller))
  ;[1 1 1] Rotate Camera on Wall Run
  ;;[0.4294 0.7963 1] Rotate Left
  (if (Actor|ActorHasTag OtherActor "WallRun")
    (bind _alpha (Timeline|RotateCameraLeftTimeline Reverse)
      (:Update
        (Pawn|SetControlRotation _returnvalue (Math|Rotator|MakeRotator (Math|Float|Lerp (.roll (Transformation|GetActorRotation)) 2e+01 _alpha) (.pitch _returnvalue_2) (.yaw _returnvalue_2)))))))

(event Custom|Headbob
  (bind _returnvalue (Game|GetPlayerController 0))
  ;[0.3783 1 0.3917] Headbob Animation Logic (if Crouch = False {play WalkHeadbob} elseif {play idleHeadbob};)
  (if (and (> (Math|Vector|VectorLength (Transformation|GetVelocity)) 0.0) (Character|CanJump))
    (if (stale Input|EnhancedActionEvents|EnhancedInputActionInput_Crouch ActionValue)
      (Game|Feedback|ClientStartCameraShake _returnvalue "/Game/Blueprints/Headbob/IdleHeadbob.IdleHeadbob_C" 1.0 "CameraLocal" "0, 0, 0" :!label _label)
      (else
        (Game|Feedback|ClientStartCameraShake _returnvalue "/Game/Blueprints/Headbob/WalkHeadbob.WalkHeadbob_C" 1.0 "CameraLocal" "0, 0, 0")))
    (else
      (goto _label))))

(event Custom|StopWallRunTimeline
  ;[1 0.3176 0.2471] Wall run logic
  (Timeline|WallRunTimeline Stop
    (:Update
      (Variables|/Script/Engine.MovementComponent|SetVelocity (Variables|Character|GetCharacterMovement) (* (Variables|Default|GetPlayerDirection) 1e+03)))))

(event Custom|JumpOffWall
  ;[0.1121 1 0.6737] Jump off wall
  (if (Variables|Default|GetIsWallRunning)
    (Utilities|IsValid (Variables|Default|GetWall)
      (:Is%20Valid
        (bind _asbp_wall_for_running (Utilities|Casting|CastToBP_WallForRunning (Variables|Default|GetWall)))
        (CallFunction|StopWallRunTimeline)
        (Character|LaunchCharacter (Math|Vector|MakeVector (.x (* (* (Math|Vector|GetForwardVector (Variables|/Game/Blueprints/BP_WallForRunning.BP_WallForRunning_C|GetArrow%20Right _asbp_wall_for_running)) (Math|Integer|SelectInt 1 -1 (> (Math|Vector|DotProduct (Math|Vector|GetForwardVector (Variables|/Game/Blueprints/BP_WallForRunning.BP_WallForRunning_C|GetArrow%20Right _asbp_wall_for_running)) (- (Transformation|GetActorLocation) (Transformation|GetActorLocation (Variables|Default|GetWall)))) 0.0))) 800)) (.y (* (* (Math|Vector|GetForwardVector (Variables|/Game/Blueprints/BP_WallForRunning.BP_WallForRunning_C|GetArrow%20Right _asbp_wall_for_running)) (Math|Integer|SelectInt 1 -1 (> (Math|Vector|DotProduct (Math|Vector|GetForwardVector (Variables|/Game/Blueprints/BP_WallForRunning.BP_WallForRunning_C|GetArrow%20Right _asbp_wall_for_running)) (- (Transformation|GetActorLocation) (Transformation|GetActorLocation (Variables|Default|GetWall)))) 0.0))) 800)) 9e+02) false false)))))

(event Custom|ResetJump
  ;[0.2339 0.8497 1] Jump Logic + Hold for higher jump + Double jump (config..)
  (Utilities|FlowControl|DoN 2) ; enters at Reset
)

(event Custom|SavePlayerLocation
  (if (AI|Components|NavMovement|IsFalling (Variables|Character|GetCharacterMovement))
    _
    (else
      (Variables|Default|SetSafeLocation (Transformation|GetActorLocation))))
  (Utilities|FlowControl|Delay 1.0)
  (CallFunction|SavePlayerLocation))

(event Input|EnhancedActionEvents|EnhancedInputActionInput_MovementCTRL
  (params (ActionValue :type Vector%202D%20Structure) (ElapsedSeconds :type Float%20%28double-precision%29) (TriggeredSeconds :type Float%20%28double-precision%29) (InputAction :type Input%20Action%20Object%20Reference :default "/Game/Core/Inputs/Input_MovementCTRL.Input_MovementCTRL"))
  ;[1 0.9386 0.5852] WASD Movement logic + Camera forward movement
  (Pawn|Input|AddMovementInput (Transformation|GetActorForwardVector) (.x ActionValue) false)
  (Pawn|Input|AddMovementInput (Transformation|GetActorRightVector) (.y ActionValue) false))

(event Input|EnhancedActionEvents|EnhancedInputActionInput_LookaroundCTRL
  (params (ActionValue :type Vector%202D%20Structure) (ElapsedSeconds :type Float%20%28double-precision%29) (TriggeredSeconds :type Float%20%28double-precision%29) (InputAction :type Input%20Action%20Object%20Reference :default "/Game/Core/Inputs/Input_LookaroundCTRL.Input_LookaroundCTRL"))
  ;[1 0.9386 0.5852] Mouse Look around logic
  (Pawn|Input|AddControllerYawInput (.x ActionValue))
  (Pawn|Input|AddControllerPitchInput (* (.y ActionValue) -1.0)))

(event Input|EnhancedActionEvents|EnhancedInputActionInput_Jump
  (params (ActionValue :type Boolean) (ElapsedSeconds :type Float%20%28double-precision%29) (TriggeredSeconds :type Float%20%28double-precision%29) (InputAction :type Input%20Action%20Object%20Reference :default "/Game/Core/Inputs/Input_Jump.Input_Jump"))
  ;[0.2339 0.8497 1] Jump Logic + Hold for higher jump + Double jump (config..)
  (:Started
    (bind _counter (Utilities|FlowControl|DoN 2)
      (:Exit
        (switch int _counter
          (:1
            _)
          (:2
            _))
        (if (Variables|Default|GetIsWallRunning)
          (CallFunction|JumpOffWall)
          (else
            (Character|Jump))))))
  (:Completed
    (Character|StopJumping)))

(event Input|EnhancedActionEvents|EnhancedInputActionInput_Dash
  (params (ActionValue :type Boolean) (ElapsedSeconds :type Float%20%28double-precision%29) (TriggeredSeconds :type Float%20%28double-precision%29) (InputAction :type Input%20Action%20Object%20Reference :default "/Game/Core/Inputs/Input_Dash.Input_Dash"))
  (bind _returnvalue (Transformation|GetVelocity))
  (bind _returnvalue_2 (* _returnvalue 5.0))
  ;[0.4004 0.2456 1] Dash Logic + Cooldown (Delay)
  (:Started
    (if (not (Variables|Default|GetIsDashing))
      (Variables|Default|SetIsDashing true)
      (Character|LaunchCharacter (Math|Vector|MakeVector (.x _returnvalue_2) (.y _returnvalue_2) 0.0) false false)
      (Utilities|FlowControl|Delay 1.0)
      (Variables|Default|SetIsDashing false))))

(event Input|EnhancedActionEvents|EnhancedInputActionInput_Crouch
  (params (ActionValue :type Boolean) (ElapsedSeconds :type Float%20%28double-precision%29) (TriggeredSeconds :type Float%20%28double-precision%29) (InputAction :type Input%20Action%20Object%20Reference :default "/Game/Core/Inputs/Input_Crouch.Input_Crouch"))
  (bind _mesh (Variables|Character|GetMesh))
  (bind _mesh_2 (Variables|Character|GetMesh))
  (bind _relativelocation (Variables|/Script/Engine.SceneComponent|GetRelativeLocation _mesh_2))
  ;[1 0.2915 0.7806] Crouch Slide
  (if (Variables|Default|GetCanSlide?)
    (Variables|Default|SetCanSlide? false)
    (Components|Capsule|SetCapsuleHalfHeight (Variables|Collision|GetCapsuleComponent) (/ (Variables|Default|GetCapsuleHeight) 2.0) true)
    (Transformation|SetRelativeLocation _mesh (+ (Variables|/Script/Engine.SceneComponent|GetRelativeLocation _mesh) "0.000000,0.000000,44.000000") false false)
    (Utilities|FlowControl|Sequence
      (:then_0
        ;;[1 1 1] Length of slide before full height
        (bind _newtrack_0 (Timeline|SetCapBack PlayFromStart)
          (:Update
            (Components|Capsule|SetCapsuleHalfHeight (Variables|Collision|GetCapsuleComponent) _newtrack_0 true))
          (:Finished
            (Variables|Default|SetCanSlide? true))))
      (:then_1
        (bind _newtrack_0_2 (Timeline|SetLocationBack PlayFromStart)
          (:Update
            (Transformation|SetRelativeLocation _mesh_2 (Math|Vector|MakeVector (.x _relativelocation) (.y _relativelocation) _newtrack_0_2) false false)))))))

(event Input|EnhancedActionEvents|EnhancedInputActionInput_Grapple
  (params (ActionValue :type Boolean) (ElapsedSeconds :type Float%20%28double-precision%29) (TriggeredSeconds :type Float%20%28double-precision%29) (InputAction :type Input%20Action%20Object%20Reference :default "/Game/Core/Inputs/Input_Grapple.Input_Grapple"))
  (bind _camera (Variables|Default|GetCamera))
  (bind _returnvalue (Transformation|GetWorldLocation _camera))
  ;[1 1 1] Grappling Hook Mechanic
  (:Started
    (bind (_outhit _returnvalue_2) (Collision|LineTraceByChannel _returnvalue (+ _returnvalue (* (Math|Vector|GetForwardVector (Transformation|GetWorldRotation _camera)) 2e+03)) "TraceTypeQuery1" false 0 "ForDuration"))
    (if _returnvalue_2
      (Variables|Default|SetGrabPoint (.ImpactPoint (Collision|BreakHitResult _outhit)))
      (Variables|Default|SetisGrappling true)
      (Pawn|Components|CharacterMovement|SetMovementMode (Variables|Character|GetCharacterMovement) "MOVE_Flying" 0)
      (Rendering|SetVisibility (Variables|Default|GetCable) true false)))
  (:Completed
    (Variables|Default|SetisGrappling false)
    (Pawn|Components|CharacterMovement|SetMovementMode (Variables|Character|GetCharacterMovement) "MOVE_Falling" 0)
    (Rendering|SetVisibility (Variables|Default|GetCable) false false)))

(event EventBeginPlay
  ;[1 1 1] Event Begin Play Sequence nodes
  (Utilities|FlowControl|Sequence
    (:then_0
      ;;[0 0 0] Enhanced Input
      (Input|AddMappingContext (PlayerController|LocalPlayerSubsystems|GetEnhancedInputLocalPlayerSubsystem (Game|GetPlayerController 0)) "/Game/Core/Inputs/IMC_ProjectDiamond.IMC_ProjectDiamond" 0 "(bIgnoreAllPressedKeysUntilRelease=True,bForceImmediately=False,bNotifyUserSettings=False)"))
    (:then_1
      ;;[1 1 1] Saving Player Location
      (CallFunction|SavePlayerLocation)
      ;;[1 0.3176 0.2471] BeginPlay - enable plane constraints (WallRun)
      (Class|MovementComponent|SetPlaneConstraintEnabled (Variables|Character|GetCharacterMovement) true)
      (Variables|Default|SetOldGravityScale (Variables|/Script/Engine.CharacterMovementComponent|GetGravityScale (Variables|Character|GetCharacterMovement))))
    (:then_2
      ;;[1 1 1] Speed Timer Widget on begin play
      (bind _returnvalue (UserInterface|CreateWidget "/Game/UI/SpeedRuntimer.SpeedRuntimer_C" (Game|GetPlayerController 0)))
      (bind _output_get (Variables|Default|SetSpeedRunTimer _returnvalue))
      (UserInterface|Viewport|AddtoViewport _output_get 0))))

(event EventTick
  (params (DeltaSeconds :type Float%20%28single-precision%29))
  ;[1 1 1] Event Tick every frame
  (Utilities|FlowControl|Sequence
    (:then_0
      ;[0.3783 1 0.3917] Headbob Animation Logic (if Crouch = False {play WalkHeadbob} elseif {play idleHeadbob};)
      (CallFunction|Headbob))
    (:then_1
      ;[1 1 1] GrappleHook cont... (on event tick)
      (if (Variables|Default|GetisGrappling)
        (Variables|/Script/CableComponent.CableComponent|SetEndLocation (Variables|Default|GetCable) (Math|Transform|InverseTransformLocation (Transformation|GetActorTransform) (Variables|Default|GetGrabPoint)))
        (Physics|AddForce (Variables|Character|GetCharacterMovement) (* (Math|Vector|Normalize (+ (Math|Vector|GetUnitDirection(Vector) (Transformation|GetActorLocation) (Variables|Default|GetGrabPoint)) (* (* (Transformation|GetActorRightVector) (Class|Actor|GetInputAxisKeyValue)) 0.7))) 4e+05))))))

(event EventOnLanded
  (params (Hit :type Hit%20Result%20Structure%20%28by%20ref%29))
  ;[0.2339 0.8497 1] Jump Logic + Hold for higher jump + Double jump (config..)
  (Utilities|FlowControl|DoN 2) ; enters at Reset
)

(fn ConstructionScript)