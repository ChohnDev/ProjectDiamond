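; BP_SpiderEnemy is an enemy that spots the player's FPS character through PawnSensing and shoots projectiles at it.
; On each sighting it snaps to face the character, then waits a short random delay before spawning BP_EnemyProjectile from its Arrow component with a 2D sound.
; The Delay ignores repeat sightings while pending, so it also throttles the fire rate while the facing keeps updating.
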(event OnSeePawn(PawnSensing)
  (params (Pawn :type Pawn%20Object%20Reference))
  (Utilities|Casting|CastToBP_FPS_Character Pawn)
  (Transformation|SetActorRotation (Math|Rotator|FindLookatRotation (Transformation|GetActorLocation) (Transformation|GetActorLocation Pawn)))
  (Utilities|FlowControl|Delay (Math|Random|RandomFloatinRange 0.2 0.5))
  (Game|SpawnActorfromClass "/Game/Blueprints/BP_EnemyProjectile.BP_EnemyProjectile_C" (Transformation|GetWorldTransform (Variables|Default|GetArrow)) "AlwaysSpawn" "MultiplyWithRoot" 0 0)
  (Audio|PlaySound2D "/Game/ImportedAssets/synth.synth" 1.0 1.0 0.0 0 0))

(fn ConstructionScript)