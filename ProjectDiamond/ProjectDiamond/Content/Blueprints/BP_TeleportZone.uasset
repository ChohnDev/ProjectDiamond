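; BP_TeleportZone is a trigger volume that returns the player character to a safe location when entered.
; On overlap with its Box, it casts the other actor to BP_FPS_Character and moves it, without sweeping, to that character's own SafeLocation.
; The construction script sets the Box's world position and scale from X, Y, Height, Size and Thickness variables, with Size shared by both horizontal axes.
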(event OnComponentBeginOverlap(Box)
  (params (OverlappedComponent :type Primitive%20Component%20Object%20Reference) (OtherActor :type Actor%20Object%20Reference) (OtherComp :type Primitive%20Component%20Object%20Reference) (OtherBodyIndex :type Integer) (bFromSweep :type Boolean) (SweepResult :type Hit%20Result%20Structure%20%28by%20ref%29))
  (bind _asbp_fps_character (Utilities|Casting|CastToBP_FPS_Character OtherActor))
  (Transformation|SetActorLocation _asbp_fps_character (Variables|/Game/Blueprints/BP_FPS_Character.BP_FPS_Character_C|GetSafeLocation _asbp_fps_character) false false))

(fn ConstructionScript
  (bind _size (Variables|Default|GetSize))
  (Transformation|SetWorldTransform (Variables|Default|GetBox) (Math|Transform|MakeTransform (Math|Vector|MakeVector (Variables|Default|GetX) (Variables|Default|GetY) (Variables|Default|GetHeight)) "0, 0, 0" (Math|Vector|MakeVector _size _size (Variables|Default|GetThickness))) false false))